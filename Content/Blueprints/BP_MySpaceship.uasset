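; BP_MySpaceship is the player spaceship Blueprint, and its graph manages the score, pause and death UI.
; BeginPlay creates the score widget and adds it to the viewport.
; The Pause input toggles game pause, creating a new pause widget on pause and removing it on resume.
; The Ondead event removes the score widget and shows a death screen widget.
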(event EventBeginPlay
  (bind _returnvalue (UserInterface|CreateWidget "/Game/Blueprints/ScoreUI.ScoreUI_C"))
  (Variables|Default|SetScoreUIRef _returnvalue)
  (UserInterface|Viewport|AddtoViewport _returnvalue 0))

(event EventOndead
  (Widget|RemovefromParent (Variables|Default|GetScoreUIRef))
  (bind _returnvalue (UserInterface|CreateWidget "/Game/Blueprints/DeadUI.DeadUI_C"))
  (UserInterface|Viewport|AddtoViewport _returnvalue 0))

(event Input|ActionEvents|InputActionPause
  (params (Key :type Key%20Structure :default "None"))
  (:Pressed
    (if (Game|IsGamePaused)
      (Game|SetGamePaused false)
      (Widget|RemovefromParent (Variables|Default|GetPauseUIRef))
      (else
        (Game|SetGamePaused true)
        (bind _returnvalue (UserInterface|CreateWidget "/Game/Blueprints/PauseUI.PauseUI_C"))
        (Variables|Default|SetPauseUIRef _returnvalue)
        (UserInterface|Viewport|AddtoViewport _returnvalue 0)))))

(fn ConstructionScript)