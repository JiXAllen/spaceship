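; Enemy ship Blueprint that handles the ship's random coloring, spawn animation and explosion effect.
; SetColor picks random body and wing colors from fixed palettes, applies them through a dynamic material instance, then plays a timeline that drives actor scale.
; SpawnExplosion spawns a particle emitter at the actor's location and passes it the stored colors, so the explosion receives the ship's palette.
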(event EventSetColor
  (Variables|Default|SetBodyColorIndex (Math|Random|RandomIntegerinRange 0 3))
  (Variables|Default|SetWingColorIndex (Math|Random|RandomIntegerinRange 0 3))
  (bind _returnvalue (Rendering|Material|CreateDynamicMaterialInstance "/Game/Materials/M_Base_Ship.M_Base_Ship" "None" "None" :!class /Script/Engine.KismetMaterialLibrary))
  (Rendering|Material|SetVectorParameterValue _returnvalue "Color1" (Utilities|Select :Index (Variables|Default|GetBodyColorIndex) :Option%200 "(R=0.333542,G=0.258681,B=0.620833,A=1.000000)" :Option%201 "(R=0.598489,G=0.191250,B=0.637500,A=1.000000)" :Option%202 "(R=0.174976,G=0.479167,B=0.097489,A=1.000000)" :Option%203 "(R=0.000000,G=0.145712,B=0.762500,A=1.000000)") :!class /Script/Engine.MaterialInstanceDynamic)
  (Rendering|Material|SetVectorParameterValue _returnvalue "Color2" (Utilities|Select :Index (Variables|Default|GetWingColorIndex) :Option%200 "(R=0.700000,G=0.053932,B=0.059502,A=1.000000)" :Option%201 "(R=0.820833,G=0.631236,B=0.057826,A=1.000000)" :Option%202 "(R=0.034475,G=0.766667,B=0.711702,A=1.000000)" :Option%203 "(R=0.175000,G=0.083780,B=0.072615,A=1.000000)") :!class /Script/Engine.MaterialInstanceDynamic)
  (Variables|Default|SetPrimaryColor (Utilities|Select :Index (Variables|Default|GetBodyColorIndex) :Option%200 "(R=0.333542,G=0.258681,B=0.620833,A=1.000000)" :Option%201 "(R=0.598489,G=0.191250,B=0.637500,A=1.000000)" :Option%202 "(R=0.174976,G=0.479167,B=0.097489,A=1.000000)" :Option%203 "(R=0.000000,G=0.145712,B=0.762500,A=1.000000)"))
  (Variables|Default|SetSecondaryColor (Utilities|Select :Index (Variables|Default|GetWingColorIndex) :Option%200 "(R=0.700000,G=0.053932,B=0.059502,A=1.000000)" :Option%201 "(R=0.820833,G=0.631236,B=0.057826,A=1.000000)" :Option%202 "(R=0.034475,G=0.766667,B=0.711702,A=1.000000)" :Option%203 "(R=0.175000,G=0.083780,B=0.072615,A=1.000000)"))
  (Rendering|Material|SetMaterial (Variables|Default|GetShipMesh) 0 _returnvalue)
  (bind _scale (Timeline|SpawnScaleTimeline Play)
    (:Update
      (Transformation|SetActorScale3D (Math|Conversions|ToVector(Float) _scale)))))

(event EventSpawnExplosion
  (bind _returnvalue (Effects|SpawnEmitteratLocation "/Game/Particles/PS_Explore.PS_Explore" (Transformation|GetActorLocation)))
  (Effects|Components|ParticleSystem|SetColorParameter _returnvalue "PrimaryColor" (Variables|Default|GetPrimaryColor))
  (Effects|Components|ParticleSystem|SetColorParameter _returnvalue "SecondaryColor" (Variables|Default|GetSecondaryColor)))

(fn ConstructionScript)